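; BP_Arquero is an archer that spawns BP_Flecha arrow actors at its own location, passing each one a firing speed.
; It spawns one arrow on BeginPlay, and DispararFlecha repeats the same spawn whenever it is called.
; VelocidadFlecha sets VelocidadDisparo, the speed given to later arrows, by scaling an input speed with MultiplicadorVelocidadFlecha.
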(event `self.ReceiveBeginPlay`
  (`|SpawnActorFromClass` "/Game/BP/BP_Flecha.BP_Flecha_C" (`KismetMathLibrary.MakeTransform` (`self.K2_GetActorLocation`)) "Undefined" "MultiplyWithRoot" null (`self.VelocidadDisparo`) null))

(fn `DispararFlecha`
  (`|SpawnActorFromClass` "/Game/BP/BP_Flecha.BP_Flecha_C" (`KismetMathLibrary.MakeTransform` (`self.K2_GetActorLocation`)) "Undefined" "MultiplyWithRoot" null (`self.VelocidadDisparo`) null))

(fn `UserConstructionScript`)

(fn `VelocidadFlecha`
  (params (Velocidad :type "Vector Structure"))
  (set `self.VelocidadDisparo` (* Velocidad (`self.MultiplicadorVelocidadFlecha`))))